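; Player camera pawn that pans, zooms and rotates in response to input.
; Axis inputs move a desired location along the actor's forward and right vectors and adjust a clamped desired spring arm length.
; Rotation actions add a yaw step to a desired rotation on each press.
; Tick interpolates the actor transform and arm length toward these targets, seeded at BeginPlay, for smooth motion.
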(event `self.ReceiveBeginPlay`
  ;[0 0 0] At the start of the game, we keep a snap of the current state of the camera as our starting point.
  (set `self.Location_Desired` (`self.K2_GetActorLocation`))
  (set `self.Zoom_Desired` (`SpringArmComponent.TargetArmLength` (`self.SpringArm`)))
  (set `self.Rotation_Desired` (`self.K2_GetActorRotation`)))

(event `self.ReceiveTick`
  (params (DeltaSeconds :type "Float (single-precision)"))
  (bind _springarm (`self.SpringArm`))
  ;[0 0 0] Every frame, we interpolate the camera movements data (to make it smoother) and apply them to the actual camera.
  (set `SpringArmComponent.TargetArmLength` (`KismetMathLibrary.FInterpTo` (`SpringArmComponent.TargetArmLength` _springarm) (`self.Zoom_Desired`) (`GameplayStatics.GetWorldDeltaSeconds`) (`self.Zoom_Interp`)) _springarm)
  (`self.K2_SetActorLocation` (`KismetMathLibrary.VInterpTo` (`self.K2_GetActorLocation`) (`self.Location_Desired`) (`GameplayStatics.GetWorldDeltaSeconds`) (`self.Location_Interp`)))
  (`self.K2_SetActorRotation` (`KismetMathLibrary.RInterpTo` (`self.K2_GetActorRotation`) (`self.Rotation_Desired`) (`GameplayStatics.GetWorldDeltaSeconds`) (`self.Rotation_Interp`))))

(event `InputAxis|InputAxis_Zoom`
  (params (AxisValue :type "Float (single-precision)"))
  ;[0 0 0] Every frame, we adding the input amount to the Zoom_Desired.
  (set `self.Zoom_Desired` (`KismetMathLibrary.FClamp` (+ (* AxisValue (`self.Zoom_Speed`)) (`self.Zoom_Desired`)) (`self.Zoom_Min`) (`self.Zoom_Max`))))

(event `InputAxis|InputAxis_X`
  (params (AxisValue :type "Float (single-precision)"))
  ;[0 0 0] Every frame, were adding the input amount to the Location_Desired. By multiplying the Foward & Right Vectors so the camera moves in the right direction.
  (set `self.Location_Desired` (+ (`self.Location_Desired`) (* (`self.GetActorForwardVector`) (* AxisValue (`self.Location_Speed`))))))

(event `InputAxis|InputAxis_Y`
  (params (AxisValue :type "Float (single-precision)"))
  ;[0 0 0] Every frame, were adding the input amount to the Location_Desired. By multiplying the Foward & Right Vectors so the camera moves in the right direction.
  (set `self.Location_Desired` (+ (`self.Location_Desired`) (* (`self.GetActorRightVector`) (* AxisValue (`self.Location_Speed`))))))

(event `InputAction|InputAction_RotationRight`
  (params (Key :type "Key Structure"))
  ;[0 0 0] Every time the player presses the inputs, we're adding the input amount to the Rotation_Desired.
  (:`Pressed`
    (set `self.Rotation_Desired` (`KismetMathLibrary.ComposeRotators` (`self.Rotation_Desired`) (`KismetMathLibrary.MakeRotator` 0.0 0.0 (- (`self.Rotation_Speed`) 0.0))))))

(event `InputAction|InputAction_RotationLeft`
  (params (Key :type "Key Structure"))
  ;[0 0 0] Every time the player presses the inputs, we're adding the input amount to the Rotation_Desired.
  (:`Pressed`
    (set `self.Rotation_Desired` (`KismetMathLibrary.ComposeRotators` (`self.Rotation_Desired`) (`KismetMathLibrary.MakeRotator` 0.0 0.0 (`self.Rotation_Speed`))))))

(fn `UserConstructionScript`)